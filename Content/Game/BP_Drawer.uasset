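; BP_Drawer is a grabbable drawer actor, apparently meant for VR, that tracks the motion controller while held.
; On grab it stores the controller's world position, then each Tick records the current position and rolls it into the previous one.
; An unconnected expression projects the position delta onto the root's forward vector for sliding, so the drawer never moves as wired.
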(event `self.ReceiveBeginPlay`
  (bind _grabcomponent (`self.GrabComponent`))
  (add `/Game/VRTemplate/Blueprints/GrabComponent.OnGrabbed` _grabcomponent (delegate `StartGrab`))
  (add `/Game/VRTemplate/Blueprints/GrabComponent.OnDropped` _grabcomponent (delegate `EndGrab`)))

(event `StartGrab`
  (set `self.PrevControllerPosition` (`SceneComponent.K2_GetComponentLocation` (`/Game/VRTemplate/Blueprints/GrabComponent.MotionControllerRef` (`self.GrabComponent`)))))

(event `EndGrab`)

(event `self.ReceiveTick`
  (params (DeltaSeconds :type "Float (single-precision)"))
  (if (`/Game/VRTemplate/Blueprints/GrabComponent.bIsHeld` (`self.GrabComponent`))
    (`|ExecutionSequence`
      (:`then_0`
        (set `self.ActualControlledPosition` (`SceneComponent.K2_GetComponentLocation` (`/Game/VRTemplate/Blueprints/GrabComponent.MotionControllerRef` (`self.GrabComponent`)))))
      (:`then_2`
        (set `self.PrevControllerPosition` (`self.ActualControlledPosition`))))))

(fn `UserConstructionScript`)