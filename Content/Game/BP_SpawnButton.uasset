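; BP_SpawnButton is an actor with a SpawnPorjectile event that spawns a BP_Projectile at the world position of its Location component.
; BeginPlay caches the player's VRPawn, though nothing shown uses it.
; The Cube's overlap event is empty.
; An unconnected chain would print "Hello" and lower the Cube each frame while overlapping-actor checks return results, but it never runs.
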(event `self.ReceiveBeginPlay`
  (bind _asvrpawn (cast `/Game/VRTemplate/Blueprints/VRPawn` (`GameplayStatics.GetPlayerPawn` 0)))
  (set `self.VRPawn` _asvrpawn))

(event `SpawnPorjectile`
  (`|SpawnActorFromClass` "/Game/Game/BP_Projectile.BP_Projectile_C" (`KismetMathLibrary.MakeTransform` (`SceneComponent.K2_GetComponentLocation` (`self. Location`))) "Undefined" "MultiplyWithRoot" null null))

(event `self.Cube.OnComponentBeginOverlap`
  (params (OverlappedComponent :type "PrimitiveComponent Object Reference") (OtherActor :type "Actor Object Reference") (OtherComp :type "PrimitiveComponent Object Reference") (OtherBodyIndex :type Integer) (bFromSweep :type Boolean) (SweepResult :type "HitResult Structure (by ref)")))

(fn `UserConstructionScript`)