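; BP_Target is a shootable target actor that explodes once when a projectile hits it.
; Its Box overlap looks for a BPC_Projectile component on the overlapping actor and, behind a DoOnce, calls that component's projectile dispatcher.
; It then hides its three cube meshes, activates the NSTargetExplode effect and destroys itself after a short delay.
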(event `self.Box.OnComponentBeginOverlap`
  (params (OverlappedComponent :type "PrimitiveComponent Object Reference") (OtherActor :type "Actor Object Reference") (OtherComp :type "PrimitiveComponent Object Reference") (OtherBodyIndex :type Integer) (bFromSweep :type Boolean) (SweepResult :type "HitResult Structure (by ref)"))
  (bind _returnvalue (`self.GetComponentByClass` OtherActor "/Game/Game/BPC_Projectile.BPC_Projectile_C"))
  (`/Engine/EditorBlueprintResources/StandardMacros.IsValid` _returnvalue
    (:`Is Valid`
      (`/Engine/EditorBlueprintResources/StandardMacros.DoOnce` false
        (:`Completed`
          (`/Game/Game/BPC_Projectile.ProjectileDispacher` _returnvalue)
          (`SceneComponent.SetHiddenInGame` (`self.Cube`) true false)
          (`SceneComponent.SetHiddenInGame` (`self.Cube1`) true false)
          (`SceneComponent.SetHiddenInGame` (`self.Cube2`) true false)
          (`ActorComponent.Activate` (`self.NS_targetExplode`) false)
          (`KismetSystemLibrary.Delay` 2.0)
          (`self.K2_DestroyActor`))))))

(fn `UserConstructionScript`)