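; BP_ViewToggle is a pressable button that toggles the VR pawn's SmoothTurn setting.
; On BeginPlay it binds both press and unpress events to the pawn's button press event.
; A timeline moves the cube along Z with a clamped offset, then reverses after a short delay.
; Timeline updates drive a FlipFlop that alternates SmoothTurn, gated by a DoOnce that resets after a delay to limit repeat toggles.
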(event `self.ReceiveBeginPlay`
  (bind _asvrpawn (cast `/Game/VRTemplate/Blueprints/VRPawn` (`GameplayStatics.GetPlayerPawn` 0)))
  (bind _output_get (set `self.VRPawn` _asvrpawn))
  (add `/Game/VRTemplate/Blueprints/VRPawn.ButtonPress` _output_get (delegate `ButtonPress`))
  (add `/Game/VRTemplate/Blueprints/VRPawn.ButtonPress` _output_get (delegate `ButtonUnpress`)))

(event `ButtonPress`
  (bind _cube (`self.Cube`))
  (bind (_relativelocation_x _relativelocation_y) (`KismetMathLibrary.BreakVector` (`SceneComponent.RelativeLocation` _cube)))
  (bind (_direction _newtrack_0) (`Timeline|ButtonRes` :!label _label)
    (:`Update`
      (`SceneComponent.K2_SetRelativeLocation` _cube (`KismetMathLibrary.MakeVector` _relativelocation_x _relativelocation_y (`KismetMathLibrary.FClamp` _newtrack_0 -20.0 0.0)) false true)
      (`/Engine/EditorBlueprintResources/StandardMacros.DoOnce` false :!label _label_2
        (:`Completed`
          (`/Engine/EditorBlueprintResources/StandardMacros.FlipFlop`
            (:`A`
              (set `/Game/VRTemplate/Blueprints/VRPawn.SmoothTurn?` true (stale `self.ReceiveBeginPlay` _output_get)))
            (:`B`
              (set `/Game/VRTemplate/Blueprints/VRPawn.SmoothTurn?` false (stale `self.ReceiveBeginPlay` _output_get))))
          (`KismetSystemLibrary.Delay` 1.5)
          (goto _label_2 :!via `Reset`))))))

(event `ButtonUnpress`
  (`KismetSystemLibrary.Delay` 0.5)
  (goto _label :!via `Reverse`))

(fn `UserConstructionScript`)